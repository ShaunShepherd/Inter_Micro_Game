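; BP_Shard is a collectible pickup that adds one shard to the first-person character on overlap and then destroys itself.
; On BeginPlay it starts placeholder spin and bob animations on its Cube component.
; Two looping timelines drive the motion: one sets yaw on the tilted cube, the other sets relative height scaled by BobHeight.
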(event `self.ReceiveBeginPlay`
  ; Start placeholder rotation and bob animations
  (bind (_direction _rotationtrack) (`Timeline|Timeline` :!label _label)
    (:`Update`
      (`SceneComponent.K2_SetRelativeRotation` (`self.Cube`) (`KismetMathLibrary.MakeRotator` 0.0 45.0 _rotationtrack) false false)
      (bind (_direction_2 _heighttrack) (`Timeline|Timeline_0` :!label _label_2)
        (:`Update`
          (`SceneComponent.K2_SetRelativeLocation` (`self.Cube`) (`KismetMathLibrary.MakeVector` 0.0 0.0 (* _heighttrack (`self.BobHeight`))) false false))
        (:`Finished`
          (goto _label_2 :!via `PlayFromStart`))))
    (:`Finished`
      (goto _label :!via `PlayFromStart`))))

(event `self.ReceiveActorBeginOverlap`
  (params (OtherActor :type "Actor Object Reference"))
  (bind _asbp_first_person_character (cast `/Game/Blueprints/BP_FirstPersonCharacter` OtherActor))
  (`/Game/Blueprints/BP_FirstPersonCharacter.CollectShards` _asbp_first_person_character 1)
  (`self.K2_DestroyActor`))

(fn `UserConstructionScript`)