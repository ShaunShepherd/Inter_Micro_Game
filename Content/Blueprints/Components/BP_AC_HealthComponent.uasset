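; Actor component that gives its owner health and destroys that owner when health runs out.
; On BeginPlay it sets Health to MaxHealth and caches the owning actor.
; A TakeDamage event subtracts the damage amount, then either destroys the owner at zero or below, or prints the remaining health.
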(event `self.ReceiveBeginPlay`
  ; Initialise health to max health
  (set `self.Health` (`self.MaxHealth`))
  ; Get a reference to the owner of this component
  (set `self.OwnerRef` (`self.GetOwner`)))

(event `TakeDamage`
  (params (DamageAmount :type "Float (double-precision)"))
  (bind _output_get (set `self.Health` (- (`self.Health`) DamageAmount)))
  (if (<= _output_get 0.0)
    (`Actor.K2_DestroyActor` (`self.OwnerRef`))
    (else
      (`KismetSystemLibrary.PrintString` (`KismetStringLibrary.Conv_DoubleToString` _output_get)))))