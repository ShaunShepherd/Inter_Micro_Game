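; BP_Tower_Sphere is a child tower Blueprint that fills in the parent's placement hooks using its Mesh component.
; On setup completion it runs the parent logic, records its own class as TowerClass and makes the mesh ignore Visibility traces.
; It applies supplied materials to the mesh's first slot and marks itself Placeable only when the mesh overlaps no actors.
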(event `/Game/Blueprints/BP_Holdable.SetupComplete`
  (`parent.SetupComplete`)
  (set `self.TowerClass` (`GameplayStatics.GetObjectClass` self))
  (`PrimitiveComponent.SetCollisionResponseToChannel` (`self.Mesh`) "ECC_Visibility" "ECR_Ignore"))

(event `self.SetMaterials`
  (params (Material :type "Material Object Reference"))
  (`PrimitiveComponent.SetMaterial` (`self.Mesh`) 0 Material))

(event `self.CheckIfPlaceable`
  (set `self.Placeable` (== (`KismetArrayLibrary.Array_Length` (`PrimitiveComponent.GetOverlappingActors` (`self.Mesh`) null)) 0)))

(fn `UserConstructionScript`
  (`parent.UserConstructionScript`))