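; BP_Tower is a base Blueprint for a tower placement preview that spends the player's Shards to build a tower.
; Each tick it checks affordability and, through the CheckIfPlaceable hook, placement validity, then applies the placeable or unplaceable material.
; LinetraceTest spawns TowerClass at the preview's transform and deducts PlacementCost when placement is allowed.
; Subclasses implement the placement check and material swap.
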(event `self.LinetraceTest`
  (params (ImpactPoint :type "Vector Structure") (ImpactNormal :type "Vector Structure") (ActorHit :type "Actor Object Reference"))
  (bind _playerref (`self.PlayerRef`))
  ; Place tower if possible
  (if (`self.Placeable`)
    (if (>= (`/Game/Blueprints/BP_FirstPersonCharacter.Shards` (`self.PlayerRef`)) (`self.PlacementCost`))
      (`|SpawnActorFromClass` (`self.TowerClass`) (`self.GetTransform`) "Undefined" "MultiplyWithRoot" null null)
      (set `/Game/Blueprints/BP_FirstPersonCharacter.Shards` (- (`/Game/Blueprints/BP_FirstPersonCharacter.Shards` _playerref) (`self.PlacementCost`)) _playerref))))

(event `self.ReceiveTick`
  (params (DeltaSeconds :type "Float (single-precision)"))
  (bind _playerref (`self.PlayerRef`))
  ; See If Tower can be placed
  (`/Engine/EditorBlueprintResources/StandardMacros.IsValid` _playerref
    (:`Is Valid`
      (if (>= (`/Game/Blueprints/BP_FirstPersonCharacter.Shards` _playerref) (`self.PlacementCost`))
        (`self.CheckIfPlaceable`)
        (if (`self.Placeable`)
          (`self.SetMaterials` (`self.PlaceableMaterial`))
          (else
            (`self.SetMaterials` (`self.UnplaceableMaterial`) :!label _label)))
        (else
          (goto _label))))))

(event `CheckIfPlaceable`
  ; Implemented by subclass to see if tower can be placed
)

(event `SetMaterials`
  (params (Material :type "Material Object Reference"))
  ; Implemented by subclasses to change tower material
)

(fn `UserConstructionScript`
  (`parent.UserConstructionScript`))