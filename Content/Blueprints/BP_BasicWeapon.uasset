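; BP_BasicWeapon is an automatic weapon actor that instantly destroys any BP_BasicEnemy it hits.
; A Timeline starts on BeginPlay and replays each time it finishes, acting as a repeating fire timer with no input or targeting.
; Each cycle fires a debug-drawn Visibility line trace from the Cube along its forward vector out to Range, then destroys the hit actor if it casts to the enemy class.
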(event `self.ReceiveBeginPlay`
  (bind _cube (`self.Cube`))
  (bind _returnvalue (`SceneComponent.K2_GetComponentLocation` _cube))
  (`Timeline|Timeline` :`NewTime` 0.0 :!via `PlayFromStart` :!label _label
    (:`Finished`
      (bind _outhit (`KismetSystemLibrary.LineTraceSingle` :`Start` _returnvalue :`End` (+ _returnvalue (* (`KismetMathLibrary.GetForwardVector` (`SceneComponent.K2_GetComponentRotation` _cube)) (`self.Range`))) :`TraceChannel` "TraceTypeQuery1" :`DrawDebugType` "ForDuration" :`TraceColor` (struct :`R` 1.0 :`G` 1.0 :`B` 1.0 :`A` 1.0) :`TraceHitColor` (struct :`R` 1.0 :`G` 1.0 :`B` 1.0 :`A` 1.0) :`DrawTime` 0.1))
      (bind _asbp_basic_enemy (cast `/Game/Blueprints/BP_BasicEnemy` (`.HitActor` (`GameplayStatics.BreakHitResult` _outhit)))
        (:`then`
          (`self.K2_DestroyActor` _asbp_basic_enemy)
          (goto _label :!via `PlayFromStart`))
        (:`CastFailed`
          (goto _label :!via `PlayFromStart`))))))

(fn `UserConstructionScript`)