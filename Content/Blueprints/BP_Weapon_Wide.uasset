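; BP_Weapon_Wide is a placeable weapon variant that fires bullets from its barrel.
; Setup extends the parent's logic by recording its class and mesh parent, and a material setter recolors the cube and barrel meshes.
; Placement is blocked while its sphere overlaps any BP_Weapon actor.
; Shooting spawns a bullet at the barrel and passes it scale, damage and a velocity along the barrel's negated forward vector.
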(event `/Game/Blueprints/BP_Holdable.SetupComplete`
  (`parent.SetupComplete`)
  (set `self.WeaponClass` (`GameplayStatics.GetObjectClass` self))
  (set `self.MeshParentRef` (`self.MeshParent`)))

(event `self.SetMaterials`
  (params (Material :type "Material Object Reference"))
  (`PrimitiveComponent.SetMaterial` (`self.Cube1`) 0 Material)
  (`PrimitiveComponent.SetMaterial` (`self.Barrel`) 0 Material))

(event `self.CheckIfPlaceable`
  ; Handle checking if placeable
  (if (> (`KismetArrayLibrary.Array_Length` (`PrimitiveComponent.GetOverlappingActors` (`self.Sphere`) "/Game/Blueprints/BP_Weapon.BP_Weapon_C")) 0)
    (set `self.Placeable` false)
    (else
      (set `self.Placeable` true))))

(event `self.Shoot`
  (bind _returnvalue (`|SpawnActorFromClass` (`self.Bullet`) (`SceneComponent.K2_GetComponentToWorld` (`self.Barrel`)) "Undefined" "MultiplyWithRoot" null null))
  (`/Game/Blueprints/BP_Bullet.SetUpInitialValues` _returnvalue 0.75 1.0 (* (`KismetMathLibrary.GetForwardVector` (`SceneComponent.K2_GetComponentRotation` (`self.Barrel`))) -2000.0))
  (`KismetSystemLibrary.PrintString` "SHOOT"))

(fn `UserConstructionScript`
  (`parent.UserConstructionScript`))