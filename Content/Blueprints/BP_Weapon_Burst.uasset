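; Placeable burst-fire weapon that fires a set number of projectiles along its barrel's forward vector on each Shoot.
; Shoot resets the burst counter and replays a Timeline scaled by BurstRate as a timer, calling BurstFire on each finish until the count runs out.
; Each shot calls FireProjectile and draws a debug line trace as placeholder GFX.
; It also sets mesh materials and blocks placement when its sphere overlaps a BP_Weapon.
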(event `/Game/Blueprints/BP_Holdable.SetupComplete`
  (`parent.SetupComplete`)
  (set `self.WeaponClass` (`GameplayStatics.GetObjectClass` self))
  (set `self.MeshParentRef` (`self.MeshParent`)))

(event `self.SetMaterials`
  (params (Material :type "Material Object Reference"))
  (`PrimitiveComponent.SetMaterial` (`self.Cube1`) 0 Material)
  (`PrimitiveComponent.SetMaterial` (`self.Barrel`) 0 Material))

(event `self.CheckIfPlaceable`
  ; Handle checking if placeable
  (if (> (`KismetArrayLibrary.Array_Length` (`PrimitiveComponent.GetOverlappingActors` (`self.Sphere`) "/Game/Blueprints/BP_Weapon.BP_Weapon_C")) 0)
    (set `self.Placeable` false)
    (else
      (set `self.Placeable` true))))

(event `self.Shoot`
  (`|ExecutionSequence`
    (:`then_0`
      (`TimelineComponent.SetPlayRate` (`self.Timeline`) (/ 1.0 (`self.BurstRate`))))
    (:`then_1`
      (set `self.BurstCounter` (`self.BurstCount`))
      (`Timeline|Timeline` :!via `PlayFromStart` :!label _label
        (:`Finished`
          (if (> (`self.BurstCounter`) 0)
            (`self.BurstFire`)
            (goto _label :!via `PlayFromStart`)))))))

(event `BurstFire`
  (bind _bulletspawn (`self.BulletSpawn`))
  (bind _returnvalue (`SceneComponent.K2_GetComponentLocation` _bulletspawn))
  (`self.FireProjectile` (`SceneComponent.K2_GetComponentToWorld` (`self.BulletSpawn`)) (`self.Range`) (`self.BulletSize`) (`self.DamagePerBullet`) (`KismetMathLibrary.GetForwardVector` (`SceneComponent.K2_GetComponentRotation` (`self.Barrel`))) (`self.BulletSpeed`))
  (`KismetSystemLibrary.LineTraceSingle` :`Start` _returnvalue :`End` (+ _returnvalue (* (`KismetMathLibrary.GetForwardVector` (`SceneComponent.K2_GetComponentRotation` _bulletspawn)) (/ (`self.Range`) 10.0))) :`TraceChannel` "TraceTypeQuery1" :`DrawDebugType` "ForDuration" :`TraceColor` (struct :`R` 1.0 :`G` 1.0 :`B` 1.0 :`A` 1.0) :`TraceHitColor` (struct :`R` 1.0 :`G` 1.0 :`B` 1.0 :`A` 1.0) :`DrawTime` 0.1)
  (set `self.BurstCounter` (- (`self.BurstCounter`) 1)))

(fn `Burst`)

(fn `UserConstructionScript`
  (`parent.UserConstructionScript`))