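; Base actor for items the player holds, with empty hooks for linetrace results, active toggling and post-setup logic.
; The inventory manager initialises it, attaching it to the player's CineCamera at a given hold position, facing the player's location.
; Setup then switches it off and fires SetupComplete.
; The player controller drives the linetrace and toggle events, for child Blueprints to implement.
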(event `InitialiseHoldable`
  (params (PlayerRef :type "/Game/Blueprints/BP_FirstPersonCharacter Object Reference") (HoldPos :type "Vector Structure"))
  ; Called when the inventroy manager sets everything up
  (bind _output_get (set `self.PlayerRef` PlayerRef))
  (`self.K2_AttachToComponent` (`/Game/Blueprints/BP_FirstPersonCharacter.CineCamera` _output_get) "None" "KeepRelative" "KeepRelative" "KeepRelative")
  (`self.K2_SetActorLocation` HoldPos false true)
  (`self.K2_SetActorRotation` (`KismetMathLibrary.MakeRotationFromAxes` (- (`self.K2_GetActorLocation` (`self.PlayerRef`)) (`self.K2_GetActorLocation`))))
  (`self.ToggleActive` false)
  (`self.SetupComplete`))

(event `LinetraceTest`
  (params (ImpactPoint :type "Vector Structure") (ImpactNormal :type "Vector Structure") (ActorHit :type "Actor Object Reference"))
  ; The player controller calls this when the linetrace is fired
)

(event `ToggleActive`
  (params (On :type Boolean))
  ; Toggles when the player controller changes active holdeable
)

(event `SetupComplete`
  ; Called after it has been initialised
)

(fn `UserConstructionScript`)