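; BP_BasicEnemy is a basic enemy that travels in relation to the Obelisk and damages it on overlap.
; On BeginPlay it caches player and game mode, then sets a flat projectile velocity from normalized (own location minus ObeliskPos) times MoveSpeed, so only a negative speed heads inward.
; A self-restarting Timeline spins its root in yaw.
; Overlapping the Obelisk applies damage through a component, triggers DestroyWithShard and destroys the actor.
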(event `self.ReceiveBeginPlay`
  ; Get reference to player blueprint
  (bind _asbp_first_person_character (cast `/Game/Blueprints/BP_FirstPersonCharacter` (`GameplayStatics.GetPlayerCharacter` 0)))
  (set `self.PlayerRef` _asbp_first_person_character)
  ; Get reference to game mode
  (bind _asbp_first_person_game_mode (cast `/Game/Blueprints/BP_FirstPersonGameMode` (`GameplayStatics.GetGameMode`)))
  (bind _output_get (set `self.GameModeRef` _asbp_first_person_game_mode))
  (bind (_returnvalue_x _returnvalue_y) (`KismetMathLibrary.BreakVector` (* (`KismetMathLibrary.Normal` (- (`self.K2_GetActorLocation`) (`/Game/Blueprints/BP_FirstPersonGameMode.ObeliskPos` _output_get))) (`self.MoveSpeed`))))
  (set `MovementComponent.Velocity` (`KismetMathLibrary.MakeVector` _returnvalue_x _returnvalue_y) (`self.ProjectileMovement`))
  (bind (_direction _rotationtrack) (`Timeline|Timeline` :!label _label)
    (:`Update`
      (`SceneComponent.K2_SetRelativeRotation` (`self.DefaultSceneRoot`) (`KismetMathLibrary.MakeRotator` 0.0 0.0 _rotationtrack) false false))
    (:`Finished`
      (goto _label :!via `PlayFromStart`))))

(event `self.ReceiveActorBeginOverlap`
  (params (OtherActor :type "Actor Object Reference"))
  (bind _asbp_obelisk (cast `/Game/Blueprints/BP_Obelisk` OtherActor))
  (`/Game/Blueprints/Components/BP_AC_DamageComponent.ApplyDamage` (`self.BP_AC_DamageComponent`) _asbp_obelisk)
  (`/Game/Blueprints/Components/BP_AC_DestroyComponent.DestroyWithShard` (`self.BP_AC_DestroyComponent`))
  (`self.K2_DestroyActor`))

(fn `UserConstructionScript`)