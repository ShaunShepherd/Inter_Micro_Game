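; BP_BasicEnemySpawner is an actor meant to spawn enemies around the obelisk, though its spawning logic is currently disconnected.
; BeginPlay caches the first-person game mode, which supplies the obelisk position.
; The unwired timer logic would periodically spawn EnemyBP, using random-angle cosine and sine offsets scaled by SpawnRadius and a random height.
; Tick is empty, so nothing spawns.
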(event `self.ReceiveBeginPlay`
  (bind _asbp_first_person_game_mode (cast `/Game/Blueprints/BP_FirstPersonGameMode` (`GameplayStatics.GetGameMode`)))
  (set `self.GameModeRef` _asbp_first_person_game_mode))

(event `self.ReceiveTick`
  (params (DeltaSeconds :type "Float (single-precision)")))

(fn `UserConstructionScript`)